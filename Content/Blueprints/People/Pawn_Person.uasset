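; Pawn_Person is a selectable person pawn, controlled by an AI_Person controller.
; SelectMyActor and DeselectMyActor show or hide the SelectedDecal, then set IsSelectedFlag on that controller to match, if the cast succeeds.
; Selection state lives on the controller, while the pawn's IsSelected function is a stub that always returns false.
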(event EventBeginPlay)

(event Collision|EventActorBeginOverlap
  (params (OtherActor :type Actor%20Object%20Reference)))

(event EventSelectMyActor
  (Rendering|SetVisibility (Variables|Default|GetSelectedDecal) true false)
  (bind _asai_person (Utilities|Casting|CastToAI_Person (Pawn|GetController)))
  (Variables|/Game/Blueprints/People/AI_Person.AI_Person_C|SetIsSelectedFlag _asai_person true))

(event EventDeselectMyActor
  (Rendering|SetVisibility (Variables|Default|GetSelectedDecal) false false)
  (bind _asai_person (Utilities|Casting|CastToAI_Person (Pawn|GetController)))
  (Variables|/Game/Blueprints/People/AI_Person.AI_Person_C|SetIsSelectedFlag _asai_person false))

(event EventTick
  (params (DeltaSeconds :type Float%20%28single-precision%29)))

(fn ConstructionScript)

(fn IsSelected
  (return false))