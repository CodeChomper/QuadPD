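; AI controller for pedestrian NPCs that wanders its pawn between NPC_Point actors.
; After a startup delay it loops, sphere-tracing ahead of the pawn for the next point and moving to a random reachable spot beside it.
; At points flagged as junctions, or when the trace or move fails, it randomly yaws the pawn before searching again.
; A separate GoTo event moves it to a given target.
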(event Custom|GoTo
  (params (Target :type Vector))
  (AI|AIMoveTo 0 Target 0 5.0 false))

(event Custom|NextPoint
  (bind _returnvalue (Pawn|GetControlledPawn))
  (bind _returnvalue_2 (Transformation|GetActorLocation _returnvalue))
  (bind _returnvalue_3 (Transformation|GetActorForwardVector _returnvalue))
  (bind _returnvalue_4 (* _returnvalue_3 1e+03))
  (bind _returnvalue_5 (+ _returnvalue_2 _returnvalue_4))
  (if (Variables|Default|GetOnJunction)
    (Variables|Default|SetOnJunction false)
    (CallFunction|RandomTurn :!label _label)
    (Utilities|FlowControl|Delay 0.2)
    (else
      (bind (_outhit _returnvalue_6) (Collision|SphereTraceForObjects _returnvalue_5 (+ _returnvalue_5 _returnvalue_4) 5e+02 (Utilities|Array|MakeArray "ObjectTypeQuery7") false 0 "None"))
      (if _returnvalue_6
        (bind _asnpc_point (Utilities|Casting|CastToNPC_Point (.HitActor (Collision|BreakHitResult _outhit))))
        (Variables|Default|SetOnJunction (Variables|/Game/Blueprints/People/NPC_Point.NPC_Point_C|GetJunction _asnpc_point))
        (AI|AIMoveTo 0 (.RandomLocation (AI|Navigation|GetRandomReachablePointinRadius (.ImpactPoint (Collision|BreakHitResult _outhit)) 4e+01 0 0)) 0 5e+01 false
          (:OnSuccess
            _)
          (:OnFail
            (goto _label)))
        (else
          (goto _label)))))
  (CallFunction|NextPoint))

(event EventBeginPlay
  (Utilities|FlowControl|Delay 5.0)
  (CallFunction|NextPoint))

(event EventTick
  (params (DeltaSeconds :type Float%20%28single-precision%29)))

(fn ConstructionScript)

(fn RandomTurn
  (bind _returnvalue (Pawn|GetControlledPawn))
  (Transformation|SetActorRotation _returnvalue (Math|Rotator|CombineRotators (Transformation|GetActorRotation _returnvalue) (Math|Rotator|MakeRotator 0.0 0.0 (Math|Random|RandomFloatinRange -45.0 45.0)))))