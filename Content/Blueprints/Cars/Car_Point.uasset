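; Car_Point is a waypoint actor for cars that links to possible next points and doubles as a random spawn location.
; On BeginPlay it has a one-in-six chance to spawn an AI-controlled Pawn_Car slightly above itself.
; Its construction script flushes debug lines, then redraws every Car_Point's links to its valid PosibleNextPoints, visualizing the whole network whenever a point is constructed.
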(event EventBeginPlay
  (bind _returnvalue (Transformation|GetActorTransform))
  (switch int (Math|Random|RandomIntegerinRange 0 5)
    (:0
      (AI|SpawnAIFromClass "/Game/Blueprints/Cars/Pawn_Car.Pawn_Car_C" 0 (+ (.location _returnvalue) "0,0,500.000000") (.rotation _returnvalue) false 0))))

(event Collision|EventActorBeginOverlap
  (params (OtherActor :type Actor%20Object%20Reference)))

(event EventTick
  (params (DeltaSeconds :type Float%20%28single-precision%29)))

(fn ConstructionScript
  (Rendering|Debug|FlushPersistentDebugLines)
  (bind _outactors (Actor|GetAllActorsOfClass "Car_Point_C"))
  (for _array_element _outactors
    (if (> (Utilities|Array|Length (Variables|Car_Point_C|GetPosibleNextPoints _array_element)) 0)
      (for _array_element_2 (Variables|Car_Point_C|GetPosibleNextPoints _array_element)
        (if (Utilities|IsValid _array_element_2)
          (Rendering|Debug|DrawDebugLine (Transformation|GetWorldLocation (Variables|Car_Point_C|GetBox _array_element)) (Transformation|GetWorldLocation (Variables|Car_Point_C|GetBox _array_element_2)) "(R=0.958333,G=0.082141,B=0.000000,A=1.000000)" 1e+03 1e+01))))))