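; AI controller that drives a car pawn along a graph of Car_Point waypoints.
; After a short delay, a sphere trace around the pawn finds a starting point, then NextPoint recursively moves to random linked points, polling instead while IsSelectedCarFlag is set.
; The random pick re-evaluates on arrival, so the stored point can differ from the one reached.
; A failed waypoint move only prints a message and ends the loop.
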(event Custom|NextPoint
  (if (Variables|Default|GetIsSelectedCarFlag)
    (Utilities|FlowControl|Delay 1.0)
    (CallFunction|NextPoint)
    (elif (not (not (Utilities|IsValid (Variables|Default|GetCurrPoint))))
      (if (not (< (Utilities|Array|Length (Variables|/Game/Blueprints/Cars/Car_Point.Car_Point_C|GetPosibleNextPoints (Variables|Default|GetCurrPoint))) 1))
        (AI|AIMoveTo 0 (Transformation|GetActorLocation (.OutItem (Utilities|Array|Random (Variables|/Game/Blueprints/Cars/Car_Point.Car_Point_C|GetPosibleNextPoints (Variables|Default|GetCurrPoint))))) 0 1.5e+02 true
          (:OnSuccess
            (Variables|Default|SetCurrPoint (.OutItem (Utilities|Array|Random (Variables|/Game/Blueprints/Cars/Car_Point.Car_Point_C|GetPosibleNextPoints (Variables|Default|GetCurrPoint)))))
            (CallFunction|NextPoint))
          (:OnFail
            (Development|PrintString "I Crashed")))))))

(event EventBeginPlay
  (bind _returnvalue (Pawn|GetControlledPawn))
  (bind _returnvalue_2 (Transformation|GetActorLocation _returnvalue))
  (bind _returnvalue_3 (Transformation|GetActorForwardVector _returnvalue))
  (bind _returnvalue_4 (* _returnvalue_3 ""))
  (bind _returnvalue_5 (+ _returnvalue_2 _returnvalue_4))
  (Utilities|FlowControl|Delay 1.0)
  (bind (_outhit _returnvalue_6) (Collision|SphereTraceForObjects _returnvalue_5 (+ _returnvalue_5 _returnvalue_4) 8e+02 (Utilities|Array|MakeArray "ObjectTypeQuery8") false 0 "None"))
  (if _returnvalue_6
    (AI|AIMoveTo 0 (.Location (Collision|BreakHitResult _outhit)) 0 1e+01 true
      (:OnSuccess
        (bind _ascar_point (Utilities|Casting|CastToCar_Point (.HitActor (Collision|BreakHitResult _outhit))))
        (Variables|Default|SetCurrPoint _ascar_point)
        (CallFunction|NextPoint)))))

(event EventTick
  (params (DeltaSeconds :type Float%20%28single-precision%29)))

(fn ConstructionScript)