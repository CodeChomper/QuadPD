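; QuadPD game mode that keeps a crime loop running by turning random citizens, on foot or in cars, into criminals.
; After a startup delay it caches every car and person pawn, then NewCrime re-triggers itself on a timer, flipping one random pick through SelectActorInterface.
; A Criminals list tracks them, with ArrestCriminal removing entries and GetFirstCriminal returning the first.
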(event Custom|GetAllCars
  (bind _outactors (Actor|GetAllActorsOfClass "/Game/Blueprints/Cars/Pawn_Car.Pawn_Car_C"))
  (bind _output_get (Variables|Default|SetCars _outactors))
  (Development|PrintString (Utilities|String|Append (Utilities|String|ToString(Integer) (Utilities|Array|Length _output_get)) ": Cars")))

(event Custom|GetAllPeople
  (bind _outactors (Actor|GetAllActorsOfClass "/Game/Blueprints/People/Pawn_Person.Pawn_Person_C"))
  (bind _output_get (Variables|Default|SetPeople _outactors))
  (Development|PrintString (Utilities|String|Append (Utilities|String|ToString(Integer) (Utilities|Array|Length _output_get)) ": People")))

(event Custom|NewCrime
  (bind _criminals (Variables|Default|GetCriminals))
  (Development|PrintString (Utilities|String|Append "Total Number of Criminals: " (Utilities|String|ToString(Integer) (Utilities|Array|Length (Variables|Default|GetCriminals)))) true true "(R=0.000000,G=0.660000,B=1.000000,A=1.000000)" 1e+01)
  (switch int (Math|Random|RandomIntegerinRange 0 1)
    (:0
      (bind _asselect_actor_interface (Utilities|Casting|CastToSelectActorInterface (.OutItem (Utilities|Array|Random (Variables|Default|GetPeople)))))
      (Default|SetIsCitizen _asselect_actor_interface false)
      (Utilities|Array|Add _criminals _asselect_actor_interface))
    (:1
      (bind _asselect_actor_interface_2 (Utilities|Casting|CastToSelectActorInterface (.OutItem (Utilities|Array|Random (Variables|Default|GetCars)))))
      (Default|SetIsCitizen _asselect_actor_interface_2 false)
      (Utilities|Array|Add _criminals _asselect_actor_interface_2)))
  (Utilities|FlowControl|Delay 1e+01)
  (CallFunction|NewCrime))

(event Custom|ArrestCriminal
  (params (Criminal :type Select%20Actor%20Interface%20Interface))
  (Utilities|Array|RemoveItem (Variables|Default|GetCriminals) Criminal))

(event EventBeginPlay
  (Utilities|FlowControl|Delay 2.0)
  (CallFunction|GetAllCars)
  (CallFunction|GetAllPeople)
  (Utilities|FlowControl|Delay 1e+01)
  (CallFunction|NewCrime))

(event EventTick
  (params (DeltaSeconds :type Float%20%28single-precision%29)))

(fn ConstructionScript)

(fn GetFirstCriminal
  (return (Utilities|Array|Get(acopy) (Variables|Default|GetCriminals))))