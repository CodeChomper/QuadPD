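; Engine component that acts as a thruster, pushing its owner's physics root along the component's up vector at its own world location.
; AddForce accumulates thrust requests, which Tick scales by delta time, applies and then clears.
; Stabalize feeds a PID calculation on world height versus desired altitude, negated and scaled by a multiplier, into AddForce.
; A debug line helper for forces is defined but not called here.
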(event EventBeginPlay
  (bind _asprimitive_component (Utilities|Casting|CastToPrimitiveComponent (Variables|/Script/Engine.Actor|GetRootComponent (Components|GetOwner))))
  (Variables|Default|SetPhysicsBody _asprimitive_component))

(event EventTick
  (params (DeltaSeconds :type Float%20%28single-precision%29))
  (CallFunction|ApplyForces DeltaSeconds))

(fn AddForce
  (params (Force :type Float%20%28double-precision%29))
  (Variables|Default|SetForcePerTick (+ Force (Variables|Default|GetForcePerTick))))

(fn ApplyForces
  (params (DeltaTime :type Float%20%28double-precision%29))
  (LocalVariables|SetpForce (* DeltaTime (Variables|Default|GetForcePerTick)))
  (CallFunction|ApplyForce (* (Math|Vector|GetUpVector) (LocalVariables|GetpForce)))
  (Variables|Default|SetForcePerTick 0.0))

(fn ApplyForce
  (params (ForceAmount :type Vector))
  (Class|PrimitiveComponent|AddForceatLocation (Variables|Default|GetPhysicsBody) ForceAmount (Transformation|GetWorldLocation) "None"))

(fn DrawDebugForce
  (params (ForceLocation :type Vector) (ForceAmount :type Vector))
  (Rendering|Debug|DrawDebugLine ForceLocation (+ ForceLocation ForceAmount) "(R=0.261828,G=1.000000,B=0.000000,A=1.000000)" 0.0 0.0))

(fn Stabalize
  (params (DiseredAltitude :type Float%20%28double-precision%29) (DeltaTime :type Float%20%28double-precision%29))
  (bind _outforce (CallFunction|PIDCalculation (.z (Transformation|GetWorldLocation)) DiseredAltitude 0.5 0.5 0.2 0.0 DeltaTime (Variables|Default|GetIntegral) (Variables|Default|GetErrorPrior)))
  (CallFunction|AddForce (* (* _outforce -1.0) (Variables|Default|GetStabilizerForceMultiplier))))